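; MrRich_BP is a Blueprint in the Character folder whose only scripted behavior is switching levels with number-key hotkeys.
; Several number keys each open a hard-coded map by name, such as Houses, desert, graveyard and hell.
; Four further Open Level nodes are unconnected with no level set, and the construction script is empty.
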(event `Key|One`
  (params (Key :type "Key Structure" :default "AnyKey"))
  (:`Pressed`
    (`GameplayStatics.OpenLevel` "Houses")))

(event `Key|Two`
  (params (Key :type "Key Structure" :default "AnyKey"))
  (:`Pressed`
    (`GameplayStatics.OpenLevel` "LHS_part1")))

(event `Key|Three`
  (params (Key :type "Key Structure" :default "AnyKey"))
  (:`Pressed`
    (`GameplayStatics.OpenLevel` "CASEY_THROWBACK_ALLYWAYPARKOUR")))

(event `Key|Four`
  (params (Key :type "Key Structure" :default "AnyKey")))

(event `Key|Five`
  (params (Key :type "Key Structure" :default "AnyKey"))
  (:`Pressed`
    (`GameplayStatics.OpenLevel` "desert")))

(event `Key|Six`
  (params (Key :type "Key Structure" :default "AnyKey")))

(event `Key|Seven`
  (params (Key :type "Key Structure" :default "AnyKey")))

(event `Key|Eight`
  (params (Key :type "Key Structure" :default "AnyKey")))

(event `Key|Nine`
  (params (Key :type "Key Structure" :default "AnyKey"))
  (:`Pressed`
    (`GameplayStatics.OpenLevel` "graveyard")))

(event `Key|Zero`
  (params (Key :type "Key Structure" :default "AnyKey"))
  (:`Pressed`
    (`GameplayStatics.OpenLevel` "hell")))

(fn `UserConstructionScript`)